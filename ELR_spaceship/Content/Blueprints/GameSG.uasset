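; GameSG is a save-game data container for the player's pawn, style index, high score, currency and material.
; The AddSaveGameData event overwrites all of these stored variables in one call, and GetData returns them together.
; It only holds the data, with no validation or disk save and load logic of its own.
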(event Custom|Add%20SaveGameData
  (params (PlayerPawn :type Player%20Plane%20Class%20Reference) (Style%20Index :type Integer) (HighScore :type Integer) (Currentcy :type Integer) (Player%20Mat :type Material%20Instance%20Object%20Reference))
  (Variables|Default|SetPlayerPawn PlayerPawn)
  (Variables|Default|SetStyle%20Index Style%20Index)
  (Variables|Default|SetHighScore HighScore)
  (Variables|Default|SetCurrentcy Currentcy)
  (Variables|Default|SetPlayer%20Mat Player%20Mat))

(fn GetData
  (return (Variables|Default|GetPlayerPawn) (Variables|Default|GetStyle%20Index) (Variables|Default|GetHighScore) (Variables|Default|GetCurrentcy) (Variables|Default|GetPlayer%20Mat)))