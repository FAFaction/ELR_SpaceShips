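; PlaneLane is a course lane segment that populates itself with enemy planes and scenery for the player's plane.
; On BeginPlay, if enabled, it rolls up to two enemy planes at left, middle or right arrows, using CourseSpawnner's odds, and randomly adds enemy or ally background ships as child actors.
; Player overlap with its box tells CourseSpawnner to spawn and remove lanes and speeds up the plane.
; A cleanup event destroys valid stored references.
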(event OnComponentBeginOverlap(Box)
  (params (OverlappedComponent :type Primitive%20Component%20Object%20Reference) (OtherActor :type Actor%20Object%20Reference) (OtherComp :type Primitive%20Component%20Object%20Reference) (OtherBodyIndex :type Integer) (bFromSweep :type Boolean) (SweepResult :type Hit%20Result%20Structure%20%28by%20ref%29))
  (bind _asplayer_plane (Utilities|Casting|CastToPlayer_Plane OtherActor))
  (bind _outactors (Actor|GetAllActorsOfClass "/Game/Blueprints/CourseSpawnner.CourseSpawnner_C"))
  (Default|SpawnLanes (Utilities|Array|Get(acopy) _outactors) true)
  (Default|IncreaseSpeed _asplayer_plane)
  (Default|RemoveLane (Utilities|Array|Get(acopy) _outactors)))

(event Custom|Spawn%20BackgoundShips
  (bind _returnvalue (Math|Random|RandomBool))
  (bind _returnvalue_2 (Math|Random|RandomIntegerinRange 0 2))
  (bind _returnvalue_3 (Math|Random|RandomIntegerinRange 0 3))
  (bind _background_ally_ships (Variables|Default|GetBackground%20Ally%20Ships))
  (bind _background_enemy_ships (Variables|Default|GetBackground%20Enemy%20Ships))
  (bind _output (Utilities|Array|Get(acopy) _background_ally_ships _returnvalue_3))
  (bind _output_2 (Utilities|Array|Get(acopy) _background_enemy_ships _returnvalue_2))
  (bind _returnvalue_4 (select _returnvalue _output_2 _output))
  ;[1 1 1] Spawn Background Shiprs
  (if (Math|Random|RandomBool)
    (Utilities|FlowControl|Sequence
      (:then_0
        (if (Math|Random|RandomBool)
          (bind _returnvalue_5 (AddComponent|AddChildActorComponent true (Math|Transform|MakeTransform (Transformation|GetWorldLocation (Variables|Default|GetBackGroundShipLoc%20L)))))
          (ChildActorComponent|SetChildActorClass _returnvalue_5 _returnvalue_4)))
      (:then_1
        (if (Math|Random|RandomBool)
          (bind _returnvalue_6 (AddComponent|AddChildActorComponent true (Math|Transform|MakeTransform (Transformation|GetWorldLocation (Variables|Default|GetBackGroundShipLoc%20R)) "0,179.000000, 0")))
          (ChildActorComponent|SetChildActorClass _returnvalue_6 _returnvalue_4))))))

(event Custom|DestroyEnemy's
  (bind _enemy_1 (Variables|Default|GetEnemy%201))
  (bind _backgroundship_r (Variables|Default|GetBackGroundShip%20R))
  (bind _enemy_2 (Variables|Default|GetEnemy%202))
  (bind _backgoundship_l (Variables|Default|GetBackGoundShip%20L))
  (Utilities|FlowControl|Sequence
    (:then_0
      (Utilities|IsValid _enemy_1
        (:Is%20Valid
          (Actor|DestroyActor _enemy_1))))
    (:then_1
      (Utilities|IsValid _enemy_2
        (:Is%20Valid
          (Actor|DestroyActor _enemy_2))))
    (:then_2
      (Utilities|IsValid _backgoundship_l
        (:Is%20Valid
          (Actor|DestroyActor _backgoundship_l))))
    (:then_3
      (Utilities|IsValid _backgroundship_r
        (:Is%20Valid
          (Actor|DestroyActor _backgroundship_r))))))

(event EventBeginPlay
  (bind _returnvalue (Math|Random|RandomIntegerinRange 0 2))
  (bind _returnvalue_2 (Math|Random|RandomIntegerinRange 0 2))
  (bind _arrow_l (Variables|Default|GetArrow%20L))
  (bind _arrow_m (Variables|Default|GetArrow%20M))
  (bind _arrow_r (Variables|Default|GetArrow%20R))
  (bind _enemyplanes (Variables|Default|GetEnemyPlanes))
  (bind _returnvalue_3 (Transformation|GetWorldTransform _arrow_r))
  (bind _returnvalue_4 (Transformation|GetWorldTransform _arrow_l))
  (bind _returnvalue_5 (Transformation|GetWorldTransform _arrow_m))
  (bind _output (Utilities|Array|Get(acopy) _enemyplanes _returnvalue_2))
  (bind _returnvalue_6 (Utilities|Select :Index _returnvalue :Option%200 _returnvalue_4 :Option%201 _returnvalue_5 :Option%202 _returnvalue_3))
  (if (Variables|Default|GetSpwan%20Enemy's)
    (Utilities|FlowControl|Sequence
      (:then_0
        (bind _outactors (Actor|GetAllActorsOfClass "/Game/Blueprints/CourseSpawnner.CourseSpawnner_C"))
        (Utilities|FlowControl|Sequence
          (:then_0
            (switch int (Math|Random|RandomIntegerinRange 0 (Variables|/Game/Blueprints/CourseSpawnner.CourseSpawnner_C|GetEnemySpawns%20Our%20xamount%20of%20time (Utilities|Array|Get(acopy) _outactors)))
              (:0
                (bind _returnvalue_7 (Game|SpawnActorfromClass _output _returnvalue_6 "AdjustIfPossibleButAlwaysSpawn" 0 0))
                (Variables|Default|SetEnemy%201 _returnvalue_7))))
          (:then_1
            (switch int (Math|Random|RandomIntegerinRange 0 (Variables|/Game/Blueprints/CourseSpawnner.CourseSpawnner_C|GetEnemySpawns%20Our%20xamount%20of%20time (Utilities|Array|Get(acopy) _outactors)))
              (:0
                (bind _returnvalue_8 (Game|SpawnActorfromClass _output _returnvalue_6 "AdjustIfPossibleButAlwaysSpawn" 0 0))
                (Variables|Default|SetEnemy%202 _returnvalue_8))))))
      (:then_1
        (CallFunction|SpawnBackgoundShips)))))

(event EventEndPlay
  (params (EndPlayReason :type EEndPlayReason%20Enum :default "Destroyed"))
  (switch Utilities|FlowControl|Switch|SwitchonEEndPlayReason EndPlayReason))

(fn ConstructionScript)