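; Player plane for a three-lane endless runner: flies forward, scores over time and spawns the CourseSpawnner on play.
; A touch-gesture macro feeds swipes (or arrow keys) into one-lane banking moves and double-taps into edge-to-edge rolls via MoveComponentTo.
; IncreaseSpeed adds speed and raises the spawner's enemy setting at exact score milestones.
; GameOver explodes, pauses, banks currency and high score in Game_GI, and shows EndScreen.
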(event Custom|Game%20Over
  (bind _plane_mesh (Variables|Default|GetPlane%20Mesh))
  (bind _returnvalue (Transformation|GetWorldLocation _plane_mesh))
  (Effects|SpawnEmitteratLocation "/Game/Blueprints/BackGroundShips/P_ExplosionTrial.P_ExplosionTrial" _returnvalue)
  (Audio|PlaySoundatLocation "/Game/GameContents/Sound/Effects/Bomb_Explosion_1__1_.Bomb_Explosion_1__1_" _returnvalue)
  (Utilities|FlowControl|Delay 0.2)
  (Game|SetGamePaused true)
  (bind _asgame_gi (Utilities|Casting|CastToGame_GI (Game|GetGameInstance)))
  (Utilities|FlowControl|Sequence
    (:then_0
      (if (> (Variables|Default|GetScore) 50)
        (Default|AddCurrentcy _asgame_gi (/ (Variables|Default|GetScore) 50)))
      (Variables|Default|SetScore 0)
      (bind _returnvalue_2 (UserInterface|CreateWidget "/Game/UI/EndScreen.EndScreen_C"))
      (UserInterface|Viewport|AddtoViewport _returnvalue_2 0))
    (:then_1
      (if (> (Variables|Default|GetScore) (Variables|/Game/Blueprints/Game_GI.Game_GI_C|GetHighScore _asgame_gi))
        (Default|AddNewHighScore _asgame_gi (Variables|Default|GetScore))))))

(event Custom|Increase%20Speed
  ;[1 1 1] Enemy Spawn Rate
  (bind _outactors (Actor|GetAllActorsOfClass "/Game/Blueprints/CourseSpawnner.CourseSpawnner_C"))
  (Variables|Default|SetSpeed (+ (Variables|Default|GetSpeed) 1e+01))
  (switch name (Utilities|String|StringToName (Utilities|String|ToString(Integer) (Variables|Default|GetScore)))
    (:5000
      (bind _output_get (Variables|/Game/Blueprints/CourseSpawnner.CourseSpawnner_C|SetEnemySpawns%20Our%20xamount%20of%20time (Utilities|Array|Get(acopy) _outactors) 1))
      (Development|PrintString (Utilities|String|ToString(Integer) _output_get) true false "(R=1.000000,G=1.000000,B=0.000000,A=1.000000)" 1e+01))
    (:20000
      (bind _output_get_2 (Variables|/Game/Blueprints/CourseSpawnner.CourseSpawnner_C|SetEnemySpawns%20Our%20xamount%20of%20time (Utilities|Array|Get(acopy) _outactors) 2))
      (Development|PrintString (Utilities|String|ToString(Integer) _output_get_2) true false "(R=1.000000,G=1.000000,B=0.000000,A=1.000000)"))
    (:50000
      (Variables|/Game/Blueprints/CourseSpawnner.CourseSpawnner_C|SetEnemySpawns%20Our%20xamount%20of%20time (Utilities|Array|Get(acopy) _outactors) 3))
    (:100000
      (Variables|/Game/Blueprints/CourseSpawnner.CourseSpawnner_C|SetEnemySpawns%20Our%20xamount%20of%20time (Utilities|Array|Get(acopy) _outactors) 4))
    (:200000
      (Variables|/Game/Blueprints/CourseSpawnner.CourseSpawnner_C|SetEnemySpawns%20Our%20xamount%20of%20time (Utilities|Array|Get(acopy) _outactors) 5))))

(event Custom|Spawn%20Corse%20Generator
  (Game|SpawnActorfromClass "/Game/Blueprints/CourseSpawnner.CourseSpawnner_C" (Math|Transform|MakeTransform (+ (Transformation|GetActorLocation) (* (Transformation|GetActorForwardVector) 3e+02))) "Undefined" 0 0))

(event Custom|Add%20Score
  (Variables|Default|SetScore (+ (Variables|Default|GetScore) 1)))

(event EventBeginPlay
  (if (Variables|Default|GetIs%20Playing)
    (bind _returnvalue (UserInterface|CreateWidget "/Game/Blueprints/PlayerHUD.PlayerHUD_C"))
    (UserInterface|Viewport|AddtoViewport _returnvalue 0)
    (CallFunction|SpawnCorseGenerator)))

(event EventTick
  (params (DeltaSeconds :type Float%20%28single-precision%29))
  ;[1 1 1] Forward
  (if (Variables|Default|GetIs%20Playing)
    (Transformation|SetActorLocation (+ (Transformation|GetActorLocation) (* (Transformation|GetActorForwardVector) (* (Variables|Default|GetSpeed) (Utilities|Time|GetWorldDeltaSeconds)))) false false)
    (Utilities|FlowControl|Delay 0.1)
    (CallFunction|AddScore)))

(event Input|KeyboardEvents|Right
  (params (Key :type Key%20Structure))
  (bind _plane_mesh (Variables|Default|GetPlane%20Mesh))
  (:Pressed
    ;[1 1 1] go left/right when swipe
    (if (not (Variables|Default|GetFinished%20Moving))
      (if (< (Variables|Default|GetLane) 2)
        (Variables|Default|SetLane (+ (Variables|Default|GetLane) 1))
        (Variables|Default|SetFinished%20Moving true)
        (Components|MoveComponentTo _plane_mesh (Math|Vector|MakeVector 0.0 (.Y (Math|Vector|BreakVector (+ (Transformation|GetWorldLocation (Variables|Default|GetPlane%20Mesh)) (* (Math|Vector|GetRightVector (Variables|Default|GetCamera)) (Variables|Default|GetLane%20Distance))))) 0.0) "30.000000,-90.000000, 0" true false 0.2 true)
        (Components|MoveComponentTo _plane_mesh (Variables|/Script/Engine.SceneComponent|GetRelativeLocation (Variables|Default|GetPlane%20Mesh)) "0.000000,-90.000000, 0" true false 0.1 true)
        (Development|PrintString "Right")
        (Variables|Default|SetFinished%20Moving false)))))

(event Input|KeyboardEvents|Left
  (params (Key :type Key%20Structure))
  (bind _plane_mesh (Variables|Default|GetPlane%20Mesh))
  (:Pressed
    ;[1 1 1] go left/right when swipe
    (if (not (Variables|Default|GetFinished%20Moving))
      (if (> (Variables|Default|GetLane) 0)
        (Variables|Default|SetLane (- (Variables|Default|GetLane) 1))
        (Variables|Default|SetFinished%20Moving true)
        (Components|MoveComponentTo _plane_mesh (Math|Vector|MakeVector 0.0 (.Y (Math|Vector|BreakVector (+ (Transformation|GetWorldLocation (Variables|Default|GetPlane%20Mesh)) (* (Math|Vector|GetRightVector (Variables|Default|GetCamera)) (* (Variables|Default|GetLane%20Distance) -1.0))))) 0.0) "-30.000000,-90.000000, 0" true false 0.2 true)
        (Components|MoveComponentTo _plane_mesh (Variables|/Script/Engine.SceneComponent|GetRelativeLocation (Variables|Default|GetPlane%20Mesh)) "0.000000,-90.000000, 0" true false 0.1 true)
        (Development|PrintString "Left")
        (Variables|Default|SetFinished%20Moving false)))))

(event Input|TouchEvents|InputTouch
  (params (Location :type Vector) (FingerIndex :type ETouchIndex%20Enum))
  (bind _lane_distance (Variables|Default|GetLane%20Distance))
  (bind _plane_mesh (Variables|Default|GetPlane%20Mesh))
  (bind _plane_mesh_2 (Variables|Default|GetPlane%20Mesh))
  (bind _camera (Variables|Default|GetCamera))
  (bind _plane_mesh_3 (Variables|Default|GetPlane%20Mesh))
  (bind _plane_mesh_4 (Variables|Default|GetPlane%20Mesh))
  (bind _lane_distance_2 (Variables|Default|GetLane%20Distance))
  (bind _plane_mesh_5 (Variables|Default|GetPlane%20Mesh))
  (bind _plane_mesh_6 (Variables|Default|GetPlane%20Mesh))
  (bind _camera_2 (Variables|Default|GetCamera))
  (bind _plane_mesh_7 (Variables|Default|GetPlane%20Mesh))
  (bind _plane_mesh_8 (Variables|Default|GetPlane%20Mesh))
  (bind _returnvalue (Transformation|GetWorldLocation _plane_mesh))
  (bind _returnvalue_2 (Math|Vector|GetRightVector _camera))
  (bind _returnvalue_3 (Transformation|GetWorldLocation _plane_mesh_5))
  (bind _returnvalue_4 (Math|Vector|GetRightVector _camera_2))
  (bind _relativelocation (Variables|/Script/Engine.SceneComponent|GetRelativeLocation _plane_mesh_3))
  (bind _relativelocation_2 (Variables|/Script/Engine.SceneComponent|GetRelativeLocation _plane_mesh_7))
  (bind _relativerotation (Variables|/Script/Engine.SceneComponent|GetRelativeRotation _plane_mesh_3))
  (:Pressed
    (Utilities|TouchGesters :!label _label
      (:2x%20tap%20left
        (if (== (Variables|Default|GetLane) 2)
          (Development|PrintString "2x Left")
          ;[1 1 1] go left/right when Double Tap
          (if (not (Variables|Default|GetFinished%20Moving))
            (if (> (Variables|Default|GetLane) 0)
              (Variables|Default|SetLane (- (Variables|Default|GetLane) 2))
              (Variables|Default|SetFinished%20Moving true)
              (Components|MoveComponentTo _plane_mesh_4 (Math|Vector|MakeVector 0.0 (.Y (Math|Vector|BreakVector (+ _returnvalue (* _returnvalue_2 (* (* _lane_distance -1.0) 2.0))))) 0.0) (Math|Rotator|MakeRotator (.roll _relativerotation) -9e+01 (.yaw _relativerotation)) false false 0.2 true)
              (Audio|PlaySound2D "/Game/GameContents/Sound/Effects/Propeller_whoosh.Propeller_whoosh" 19.0)
              (Components|MoveComponentTo _plane_mesh_4 _relativelocation "0,-90.000000, 0" false false 0.3 true)
              (Development|PrintString "Left")
              (Variables|Default|SetFinished%20Moving false)))
          (else
            ;[1 1 1] go left/right when swipe
            (if (not (Variables|Default|GetFinished%20Moving)) :!label _label_2
              (if (> (Variables|Default|GetLane) 0)
                (Variables|Default|SetLane (- (Variables|Default|GetLane) 1))
                (Variables|Default|SetFinished%20Moving true)
                (Components|MoveComponentTo _plane_mesh_8 (Math|Vector|MakeVector 0.0 (.Y (Math|Vector|BreakVector (+ _returnvalue_3 (* _returnvalue_4 (* _lane_distance_2 -1.0))))) 0.0) "-30.000000,-90.000000, 0" true false 0.2 true)
                (Components|MoveComponentTo _plane_mesh_8 _relativelocation_2 "0.000000,-90.000000, 0" true false 0.1 true)
                (Development|PrintString "Left")
                (Variables|Default|SetFinished%20Moving false))))))
      (:2x%20tap%20right
        (if (== (Variables|Default|GetLane) 0)
          (Development|PrintString "2x Right")
          (if (not (Variables|Default|GetFinished%20Moving))
            (if (< (Variables|Default|GetLane) 2)
              (Variables|Default|SetLane (+ (Variables|Default|GetLane) 2))
              (Variables|Default|SetFinished%20Moving true)
              (Components|MoveComponentTo _plane_mesh_2 (Math|Vector|MakeVector 0.0 (.Y (Math|Vector|BreakVector (+ _returnvalue (* _returnvalue_2 (* _lane_distance 2.0))))) 0.0) (Math|Rotator|MakeRotator (.roll _relativerotation) 9e+01 (.yaw _relativerotation)) false false 0.2 true)
              (Audio|PlaySound2D "/Game/GameContents/Sound/Effects/Propeller_whoosh.Propeller_whoosh" 19.0)
              (Components|MoveComponentTo _plane_mesh_2 _relativelocation "0,-90.000000, 0" false false 0.3 true)
              (Development|PrintString "Right")
              (Variables|Default|SetFinished%20Moving false)))
          (else
            (if (not (Variables|Default|GetFinished%20Moving)) :!label _label_3
              (if (< (Variables|Default|GetLane) 2)
                (Variables|Default|SetLane (+ (Variables|Default|GetLane) 1))
                (Variables|Default|SetFinished%20Moving true)
                (Components|MoveComponentTo _plane_mesh_6 (Math|Vector|MakeVector 0.0 (.Y (Math|Vector|BreakVector (+ _returnvalue_3 (* _returnvalue_4 _lane_distance_2)))) 0.0) "30.000000,-90.000000, 0" true false 0.2 true)
                (Components|MoveComponentTo _plane_mesh_6 _relativelocation_2 "0.000000,-90.000000, 0" true false 0.1 true)
                (Development|PrintString "Right")
                (Variables|Default|SetFinished%20Moving false))))))
      (:Left
        (goto _label_2))
      (:Right
        (goto _label_3))))
  (:Released
    (goto _label Touch%20End)))

(fn ConstructionScript)