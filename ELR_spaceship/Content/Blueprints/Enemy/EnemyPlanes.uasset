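; Enemy plane actor that fires EnemyBullets while the player pawn is within 3000 units.
; Tick feeds a randomized Delay that sets the fire rate, then a FlipFlop alternates spawns between the left and right arrows.
; Each bullet faces along its arrow's forward vector rather than at the player, with a random machine-gun sound at the plane mesh.
; Movement and lifespan nodes are present but never run.
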(event EventTick
  (params (DeltaSeconds :type Float%20%28single-precision%29))
  (Utilities|FlowControl|Sequence
    (:then_1
      (if (< (Transformation|GetDistanceTo (Game|Player|GetPlayerPawn 0)) 3e+03)
        (Utilities|FlowControl|Delay (Math|Random|RandomFloatinRange 0.3 1.0))
        (bind _isa (Utilities|FlowControl|FlipFlop)
          (:A
            _)
          (:B
            _))
        (Game|SpawnActorfromClass "/Game/Blueprints/Enemy/EnemyBullets.EnemyBullets_C" (Math|Transform|MakeTransform (Transformation|GetWorldLocation (select _isa (Variables|Default|GetArrow%20R) (Variables|Default|GetArrow%20L))) (Math|Rotator|FindLookatRotation (Transformation|GetWorldLocation (select _isa (Variables|Default|GetArrow%20R) (Variables|Default|GetArrow%20L))) (+ (Transformation|GetWorldLocation (select _isa (Variables|Default|GetArrow%20R) (Variables|Default|GetArrow%20L))) (* (Math|Vector|GetForwardVector (select _isa (Variables|Default|GetArrow%20R) (Variables|Default|GetArrow%20L))) 9999.0)))) "Undefined" 0 0)
        (Audio|PlaySoundatLocation (Utilities|Select :Index (Math|Random|RandomIntegerinRange 0 2) :Option%200 "/Game/GameContents/Sound/Effects/Futuristic_Machine_Gun_1.Futuristic_Machine_Gun_1" :Option%201 "/Game/GameContents/Sound/Effects/Futuristic_Machine_Gun_4.Futuristic_Machine_Gun_4" :Option%202 "/Game/GameContents/Sound/Effects/Futuristic_Machine_Gun_5.Futuristic_Machine_Gun_5") (Transformation|GetWorldLocation (Variables|Default|GetPlane%20Mesh)) "0, 0, 0" 0.2)))))

(event EventBeginPlay)

(fn ConstructionScript)