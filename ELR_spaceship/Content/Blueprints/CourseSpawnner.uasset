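; Course spawner actor that builds a track by chaining PlaneLane segments end to end.
; On BeginPlay it lays an enemy-free opening stretch from its Arrow, with each new lane's SpawnTransform component setting where the next one attaches.
; SpawnLanes takes a flag for enemy spawning and records each lane in an array.
; The removelane event trims the oldest lane once the array exceeds a cap, destroying its enemies first.
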(event Custom|SpawnLanes
  (params (Spwan%20Enemy's :type Boolean))
  (Utilities|FlowControl|Sequence
    (:then_0
      (bind _returnvalue (Game|SpawnActorfromClass "/Game/Blueprints/PlaneLane.PlaneLane_C" (Variables|Default|GetLane%20Transform) "AlwaysSpawn" 0 Spwan%20Enemy's 0))
      (Utilities|Array|Add (Variables|Default|GetLanes) _returnvalue)
      (Variables|Default|SetLane%20Transform (Transformation|GetWorldTransform (Variables|/Game/Blueprints/PlaneLane.PlaneLane_C|GetSpawn%20Transform _returnvalue))))))

(event Custom|remove%20lane
  (bind _lanes (Variables|Default|GetLanes))
  (bind _output (Utilities|Array|Get(acopy) _lanes))
  (if (> (Utilities|Array|Length _lanes) 20)
    (Default|DestroyEnemy's _output)
    (Utilities|FlowControl|Delay 0.2)
    (Actor|DestroyActor _output)
    (Utilities|Array|RemoveItem _lanes _output)))

(event EventBeginPlay
  (Variables|Default|SetLane%20Transform (Transformation|GetWorldTransform (Variables|Default|GetArrow)))
  (for _index (range 0 6)
    (CallFunction|SpawnLanes false)))

(fn ConstructionScript)