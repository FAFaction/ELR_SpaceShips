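; Game instance that holds player pawn, style index, high score, currency and player material, with events to update score and currency.
; SaveGameFiles copies these values into a new GameSG object and writes it to slot "SG", and runs on Shutdown.
; Init checks that slot, but reads its values from a newly created GameSG object instead of loading the saved one.
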(event Custom|Add%20New%20HighScore
  (params (Score :type Integer))
  (Variables|Default|SetHighScore Score))

(event Custom|Save%20Game%20Files
  (bind _returnvalue (SaveGame|CreateSaveGameObject "/Game/Blueprints/GameSG.GameSG_C"))
  (Default|AddSaveGameData _returnvalue (Variables|Default|GetPlayer%20Pawn) (Variables|Default|GetStyle%20Index) (Variables|Default|GetHighScore) (Variables|Default|GetCurrentcy) (Variables|Default|GetPlayer%20Mat))
  (SaveGame|SaveGametoSlot _returnvalue "SG"))

(event Custom|Subtract%20Currentcy
  (params (Amount :type Integer))
  (Variables|Default|SetCurrentcy (- (Variables|Default|GetCurrentcy) Amount)))

(event Custom|Add%20Currentcy
  (params (Amount :type Integer))
  (Variables|Default|SetCurrentcy (+ (Variables|Default|GetCurrentcy) Amount)))

(event EventInit
  (bind _returnvalue (SaveGame|DoesSaveGameExist "SG"))
  (if _returnvalue
    (bind _returnvalue_2 (SaveGame|CreateSaveGameObject "/Game/Blueprints/GameSG.GameSG_C"))
    (bind (_playerpawn _style_index _highscore _currentcy _player_mat) (Default|GetData _returnvalue_2))
    (Variables|Default|SetPlayer%20Pawn _playerpawn)
    (Variables|Default|SetStyle%20Index _style_index)
    (Variables|Default|SetHighScore _highscore)
    (Variables|Default|SetCurrentcy _currentcy)
    (Variables|Default|SetPlayer%20Mat _player_mat)))

(event EventShutdown
  (CallFunction|SaveGameFiles))